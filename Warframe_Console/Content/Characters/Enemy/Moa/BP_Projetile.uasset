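; BP_Projetile is an enemy projectile, filed under the Moa enemy, that damages the player on overlap.
; BeginPlay caches the BP_Player found in the level.
; On actor overlap, it checks whether the player's Box overlaps its Sphere, then subtracts a small fixed amount from PlayerHealth directly and prints a debug message.
; The HitPlayer event is empty, and the file shows no movement or destruction logic.
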(event Custom|Hit%20Player)

(event EventBeginPlay
  (bind _returnvalue (Actor|GetActorOfClass "/Game/Characters/Player/BP_Player.BP_Player_C"))
  (Variables|Default|SetPlayer%20Ref _returnvalue))

(event Collision|EventActorBeginOverlap
  (params (OtherActor :type Actor%20Object%20Reference))
  (bind _player_ref (Variables|Default|GetPlayer%20Ref))
  (if (Class|PrimitiveComponent|IsOverlappingComponent (Variables|/Game/Characters/Player/BP_Player.BP_Player_C|GetBox _player_ref) (Variables|Default|GetSphere))
    (Variables|/Game/Characters/Player/BP_Player.BP_Player_C|SetPlayerHealth _player_ref (- (Variables|/Game/Characters/Player/BP_Player.BP_Player_C|GetPlayerHealth _player_ref) 0.01))
    (Development|PrintString "Hit Player")))

(event EventTick
  (params (DeltaSeconds :type Float%20%28single-precision%29)))

(fn ConstructionScript)