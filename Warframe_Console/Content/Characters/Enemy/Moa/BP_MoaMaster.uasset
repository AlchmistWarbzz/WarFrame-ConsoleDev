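; BP_MoaMaster is a stationary-logic enemy that faces the player and periodically spawns projectiles.
; BeginPlay caches player, weapon and projectile references via GetActorOfClass, then starts looping timers for shooting and turning.
; A fast timer, rather than Tick, yaws it toward the player unless the player's Box overlaps its Capsule.
; Overlapping the cached weapon while the player is attacking destroys it instantly.
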(event Custom|Shoot
  (Game|SpawnActorfromClass "/Game/Characters/Enemy/Moa/BP_Progetile.BP_Progetile_C" (Transformation|GetWorldTransform (Variables|Default|GetPrjectileLoc)) "Undefined" "MultiplyWithRoot" (Variables|Default|GetProjectile%20Ref) 0)
  (Development|PrintString "Spawned"))

(event Custom|Turning
  (bind _capsule (Variables|Default|GetCapsule))
  (bind _playerref (Variables|Default|GetPlayerRef))
  (bind _box (Variables|/Game/Characters/Player/BP_Player.BP_Player_C|GetBox _playerref))
  (bind _returnvalue (Class|PrimitiveComponent|IsOverlappingComponent _box _capsule))
  (Variables|Default|SetIsOverlapping (not _returnvalue))
  (Variables|Default|SetIsOverlapping _returnvalue)
  (if (Variables|Default|GetIsOverlapping)
    (Development|PrintString "Hello")
    (else
      (Transformation|SetActorRotation (Math|Rotator|MakeRotator 0.0 0.0 (.yaw (Math|Rotator|FindLookatRotation (Transformation|GetActorLocation) (Transformation|GetActorLocation (Variables|Default|GetPlayerRef)))))))))

(event EventBeginPlay
  ;[1 1 1] Ref for Blueprints
  (Utilities|FlowControl|Sequence
    (:then_0
      (bind _returnvalue (Actor|GetActorOfClass "/Game/Characters/Enemy/Moa/BP_Progetile.BP_Progetile_C"))
      (Variables|Default|SetProjectile%20Ref _returnvalue))
    (:then_1
      (bind _returnvalue_2 (Actor|GetActorOfClass "/Game/Characters/Player/BP_Player.BP_Player_C"))
      (Variables|Default|SetPlayerRef _returnvalue_2))
    (:then_2
      (bind _returnvalue_3 (Actor|GetActorOfClass "/Game/BP/BP_Weapon.BP_Weapon_C"))
      (Variables|Default|SetWeapon%20Ref _returnvalue_3))
    (:then_3
      ;[1 1 1] Damage
      (Utilities|Time|SetTimerbyEvent (delegate Custom|Shoot) 5.0 true))
    (:then_4
      (Utilities|Time|SetTimerbyEvent (delegate Custom|Turning) 0.01 true))))

(event Collision|EventActorBeginOverlap
  (params (OtherActor :type Actor%20Object%20Reference))
  ;[1 1 1] Damage
  (if (and (== OtherActor (Variables|Default|GetWeapon%20Ref)) (Variables|/Game/Characters/Player/BP_Player.BP_Player_C|GetIsAttacking (Variables|Default|GetPlayerRef)))
    (Actor|DestroyActor)))

(event EventTick
  (params (DeltaSeconds :type Float%20%28single-precision%29)))

(fn ConstructionScript)