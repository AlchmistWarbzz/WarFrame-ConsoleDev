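; BP_EnemyMoaBody1 is a Moa enemy body that dies when the player's weapon hits it during an attack.
; BeginPlay caches the nearest BP_EnemyMoaBody, weapon, projectile and player, and initializes health, though only the weapon and player references drive damage.
; Both Tick, via Damaged, and ActorBeginOverlap test weapon mesh overlap with OverlappingCollision while attacking.
; A hit destroys the Moa outright and calls Kills on the player.
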(event Custom|Damaged
  ;[1 1 1] Damage
  (if (and (Class|PrimitiveComponent|IsOverlappingComponent (Variables|/Game/BP/BP_Weapon.BP_Weapon_C|GetStaticMesh (Variables|Default|GetWeapon%20Ref)) (Variables|Default|GetOverlappingCollision)) (Variables|/Game/Characters/Player/BP_Player.BP_Player_C|GetIsAttacking (Variables|Default|GetPlayerRef)))
    (Actor|DestroyActor)
    (bind _returnvalue (Actor|GetActorOfClass "/Game/Characters/Player/BP_Player.BP_Player_C"))
    (Default|Kills _returnvalue)))

(event EventBeginPlay
  ;[0.7228 0.4059 1] Ref for Blueprints
  (Utilities|FlowControl|Sequence
    (:then_0
      ;;[1 0.2188 0.2188] Reference Enemies in Level
      (bind _outactors (Actor|GetAllActorsOfClass "/Game/Characters/Moa/BP_EnemyMoaBody.BP_EnemyMoaBody_C"))
      (Variables|Default|SetEnemy%20Actors (Utilities|Array|MakeArray (.ReturnValue (Actor|FindNearestActor (Transformation|GetWorldLocation (Variables|Default|GetSK_Enemy_MoaBody)) _outactors)))))
    (:then_1
      (bind _returnvalue (Actor|GetActorOfClass "/Game/BP/BP_Weapon.BP_Weapon_C"))
      (Variables|Default|SetWeapon%20Ref _returnvalue))
    (:then_2
      (bind _returnvalue_2 (Actor|GetActorOfClass "/Game/BP/BP_Projetile.BP_Projetile_C"))
      (Variables|Default|SetProjectile%20Ref _returnvalue_2))
    (:then_3
      (bind _returnvalue_3 (Actor|GetActorOfClass "/Game/Characters/Player/BP_Player.BP_Player_C"))
      (Variables|Default|SetPlayerRef _returnvalue_3))
    (:then_4
      (Variables|Default|SetMoaHealth 1.0))))

(event Collision|EventActorBeginOverlap
  (params (OtherActor :type Actor%20Object%20Reference))
  ;[1 1 1] Damage
  (if (and (Class|PrimitiveComponent|IsOverlappingComponent (Variables|/Game/BP/BP_Weapon.BP_Weapon_C|GetStaticMesh (Variables|Default|GetWeapon%20Ref)) (Variables|Default|GetOverlappingCollision)) (Variables|/Game/Characters/Player/BP_Player.BP_Player_C|GetIsAttacking (Variables|Default|GetPlayerRef)))
    (Actor|DestroyActor)
    (bind _returnvalue (Actor|GetActorOfClass "/Game/Characters/Player/BP_Player.BP_Player_C"))
    (Default|Kills _returnvalue)))

(event EventTick
  (params (DeltaSeconds :type Float%20%28single-precision%29))
  (CallFunction|Damaged))

(fn ConstructionScript)