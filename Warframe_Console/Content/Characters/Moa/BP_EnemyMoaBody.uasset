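; BP_EnemyMoaBody is the body of the Moa enemy, handling its health, death and loot drop.
; AnyDamage lowers health and, near zero, ragdolls the skeletal mesh, then once destroys the head component, reports the kill to BP_Player and randomly spawns a health pickup.
; A delay later switches physics off on the corpse.
; BeginPlay sets starting health and caches nearest-enemy, weapon, projectile and player references, which the death logic leaves unused.
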(event EventBeginPlay
  ;[0.7228 0.4059 1] Ref for Blueprints
  (Utilities|FlowControl|Sequence
    (:then_0
      ;;[1 0.2188 0.2188] Reference Enemies in Level
      (bind _outactors (Actor|GetAllActorsOfClass "BP_EnemyMoaBody_C"))
      (Variables|Default|SetEnemy%20Actors (Utilities|Array|MakeArray (.ReturnValue (Actor|FindNearestActor (Transformation|GetWorldLocation (Variables|Default|GetSK_Enemy_MoaBody)) _outactors)))))
    (:then_1
      (bind _returnvalue (Actor|GetActorOfClass "/Game/BP/BP_Weapon.BP_Weapon_C"))
      (Variables|Default|SetWeapon%20Ref _returnvalue))
    (:then_2
      (bind _returnvalue_2 (Actor|GetActorOfClass "/Game/BP/BP_Projetile.BP_Projetile_C"))
      (Variables|Default|SetProjectile%20Ref _returnvalue_2))
    (:then_3
      (bind _returnvalue_3 (Actor|GetActorOfClass "/Game/Characters/Player/BP_Player.BP_Player_C"))
      (Variables|Default|SetPlayerRef _returnvalue_3))
    (:then_4
      (Variables|Default|SetMoaHealth 35.0))))

(event EventTick
  (params (DeltaSeconds :type Float%20%28single-precision%29)))

(event Game|Damage|EventAnyDamage
  (params (Damage :type Float%20%28single-precision%29) (DamageType :type Damage%20Type%20Object%20Reference) (InstigatedBy :type Controller%20Object%20Reference) (DamageCauser :type Actor%20Object%20Reference))
  ;[1 0 0] Damage
  (Variables|Default|SetMoaHealth (- (Variables|Default|GetMoaHealth) Damage))
  (if (<= (Variables|Default|GetMoaHealth) 1.0)
    ;;[1 0 0.9516] Ragdoll
    (Physics|SetSimulatePhysics (Variables|Default|GetSK_Enemy_MoaBody) true)
    (Utilities|FlowControl|Delay 0.2)
    (Utilities|FlowControl|DoOnce false
      (:Completed
        (Components|DestroyComponent (Variables|Default|GetBP_EnemyMoaHead))
        ;;[1 0.4241 0] Panel Kill Counter
        (bind _returnvalue (Actor|GetActorOfClass "/Game/Characters/Player/BP_Player.BP_Player_C"))
        (Default|Kills _returnvalue)
        (if (Math|Random|RandomBool)
          (Utilities|FlowControl|Delay 0.2)
          (Game|SpawnActorfromClass "/Game/BP/BP_HealthPickup.BP_HealthPickup_C" (Math|Transform|MakeTransform (+ (Transformation|GetActorLocation) "0.000000,0.000000,136.828196") "0, 0, 0" "1.000000,1.000000,1.000000") "Undefined" "MultiplyWithRoot" 0 0))
        (Utilities|FlowControl|Delay 5.0)
        (Physics|SetSimulatePhysics (Variables|Default|GetSK_Enemy_MoaBody) false)))))

(fn ConstructionScript)