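; BP_MoaBoss is a Moa boss enemy that shifts between three lanes once pawn sensing spots the player.
; FollowPlayer uses nested FlipFlops to alternate shift direction for ChangeLanes, whose timelines drive AI movement, yaw toward the player and an MPC_Death material parameter.
; Tick prints health and destroys the boss when an attacking player's weapon overlaps it at near-zero health, though nothing here lowers health.
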(event OnSeePawn(PawnSensing)
  (params (Pawn :type Pawn%20Object%20Reference))
  ;[0 0.8716 1] AI Sensing
  (Utilities|Casting|CastToBP_Player Pawn)
  (Variables|Default|SetIs%20Seeing%20Player true)
  (CallFunction|FollowPlayer))

(event Custom|Change%20Lanes
  (params (Shift%20Lane :type Integer))
  (bind _returnvalue (Transformation|GetActorLocation))
  ;[0.3858 1 0.2587] Lane Movement
  (Utilities|FlowControl|Delay 2.0)
  (Variables|Default|SetTarget%20Lane (Math|Integer|Clamp(Integer) (+ Shift%20Lane (Variables|Default|GetCurrent%20Lane)) 0 2))
  (Variables|Default|SetCurrent%20Position (.Y (Math|Vector|BreakVector (Transformation|GetActorLocation))))
  (bind _newtrack_0 (Timeline|Timeline PlayFromStart)
    (:Update
      (CallFunction|Rotate)
      (AI|AIMoveTo self (Math|Vector|MakeVector (+ (.x _returnvalue) (.X (Class|KismetMathLibrary|BreakVector3f (Transformation|GetActorLocation (Variables|Default|GetPlayer%20Ref))))) (Math|Float|Lerp (Variables|Default|GetCurrent%20Position) (Utilities|Array|Get(acopy) (Variables|Default|GetLane%20Position) (Variables|Default|GetTarget%20Lane)) _newtrack_0) (.z _returnvalue)) 0 5.0 false
        (:then
          (bind _newtrack_0_2 (Timeline|Timeline_0 PlayFromStart)
            (:Update
              (Rendering|Material|SetScalarParameterValue "/Game/Materials/Textures/MPC_Death.MPC_Death" "Amount 1" _newtrack_0_2 :!class /Script/Engine.KismetMaterialLibrary)
              (CallFunction|Rotate))))))
    (:Finished
      (Variables|Default|SetCurrent%20Lane (Variables|Default|GetTarget%20Lane)))))

(event Custom|FollowPlayer
  (bind _player_ref (Variables|Default|GetPlayer%20Ref))
  ;[0.3974 0 1] Random Movement
  (if (Variables|Default|GetIs%20Seeing%20Player)
    (if (or (== (Variables|Default|GetCurrent%20Lane) (Variables|/Game/Characters/Player/BP_Player.BP_Player_C|GetTargetLane _player_ref)) (== (Variables|/Game/Characters/Player/BP_Player.BP_Player_C|GetCurrentLane _player_ref) (Variables|Default|GetCurrent%20Lane)))
      (Utilities|FlowControl|FlipFlop :!label _label
        (:A
          (Utilities|FlowControl|FlipFlop
            (:A
              (CallFunction|ChangeLanes 1 :!label _label_2))
            (:B
              (CallFunction|ChangeLanes -1 :!label _label_3))))
        (:B
          (Utilities|FlowControl|FlipFlop :!label _label_4
            (:A
              (goto _label_3))
            (:B
              (goto _label_2)))))
      (else
        (Utilities|FlowControl|FlipFlop
          (:A
            (goto _label))
          (:B
            (goto _label_4)))))))

(event Custom|Rotate
  ;[1 0.1927 0.1927] Body Face Player (May Delete)
  (Transformation|SetActorRotation (Math|Rotator|MakeRotator 0.0 0.0 (.yaw (Math|Interpolation|RInterpTo (Transformation|GetActorRotation) (Math|Rotator|FindLookatRotation (Transformation|GetActorLocation) (Transformation|GetActorLocation (Variables|Default|GetPlayer%20Ref))) (Utilities|Time|GetWorldDeltaSeconds) (Math|Random|RandomFloatinRange 2.0 3.0))))))

(event Custom|Damaged
  ;[1 0 0] Damage
  (if (Math|Boolean|ANDBoolean (Class|PrimitiveComponent|IsOverlappingComponent (Variables|Default|GetOverlappingCollision) (Variables|/Game/BP/BP_Weapon.BP_Weapon_C|GetBox (Variables|Default|GetWeapon%20Ref))) (Variables|/Game/Characters/Player/BP_Player.BP_Player_C|GetIsAttacking (Variables|Default|GetPlayer%20Ref)) (< (Variables|Default|GetMoa%20Health) 0.1))
    (Actor|DestroyActor)))

(event EventBeginPlay
  ;[0.7228 0.4059 1] Ref for Blueprints
  (Utilities|FlowControl|Sequence
    (:then_0
      ;;[1 0.2188 0.2188] Reference Enemies in Level
      (bind _returnvalue (Actor|GetActorOfClass "/Game/Characters/Moa/BP_EnemyMoaHeadBoss.BP_EnemyMoaHeadBoss_C"))
      (Variables|Default|SetBoss%20Head%20REf _returnvalue))
    (:then_1
      (Actor|GetActorOfClass "/Game/BP/BP_Weapon.BP_Weapon_C")
      (Variables|Default|SetWeapon%20Ref (Variables|Default|GetWeapon%20Ref)))
    (:then_2
      (Actor|GetActorOfClass "/Game/BP/BP_Projetile.BP_Projetile_C")
      (Variables|Default|SetProjectile%20Ref (Variables|Default|GetProjectile%20Ref)))
    (:then_3
      (bind _returnvalue_2 (Actor|GetActorOfClass "/Game/Characters/Player/BP_Player.BP_Player_C"))
      (Variables|Default|SetPlayer%20Ref _returnvalue_2))
    (:then_4
      (Variables|Default|SetMoa%20Health 1e+01))))

(event Collision|EventActorBeginOverlap
  (params (OtherActor :type Actor%20Object%20Reference)))

(event EventTick
  (params (DeltaSeconds :type Float%20%28single-precision%29))
  ;[0.5484 1 0] Tick
  (Development|PrintString (Utilities|String|ToString(Float) (Variables|Default|GetMoa%20Health)))
  (CallFunction|Damaged))

(fn ConstructionScript)