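; BP_Start is a door actor whose Cube opens and closes as the player passes through two trigger boxes.
; When BP_Player overlaps Box, the Cube slides up over one second; overlapping Box1 slides it back down by the same distance.
; Each trigger plays the Door sound at the world origin and destroys itself, so each movement fires only once.
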(event OnComponentBeginOverlap(Box1)
  (params (OverlappedComponent :type Primitive%20Component%20Object%20Reference) (OtherActor :type Actor%20Object%20Reference) (OtherComp :type Primitive%20Component%20Object%20Reference) (OtherBodyIndex :type Integer) (bFromSweep :type Boolean) (SweepResult :type Hit%20Result%20Structure%20%28by%20ref%29))
  (bind _cube (Variables|Default|GetCube))
  (Utilities|Casting|CastToBP_Player OtherActor)
  (Components|DestroyComponent (Variables|Default|GetBox1))
  (Audio|PlaySoundatLocation "/Game/SFX/Door.Door" "0, 0, 0" "0, 0, 0" 1.0 1.0 0.0 0 0 0 0)
  (Components|MoveComponentTo _cube (- (Variables|/Script/Engine.SceneComponent|GetRelativeLocation _cube) "0.000000,0.000000,300.000000") (Variables|/Script/Engine.SceneComponent|GetRelativeRotation _cube) false false 1.0 false))

(event OnComponentBeginOverlap(Box)
  (params (OverlappedComponent :type Primitive%20Component%20Object%20Reference) (OtherActor :type Actor%20Object%20Reference) (OtherComp :type Primitive%20Component%20Object%20Reference) (OtherBodyIndex :type Integer) (bFromSweep :type Boolean) (SweepResult :type Hit%20Result%20Structure%20%28by%20ref%29))
  (bind _cube (Variables|Default|GetCube))
  (Utilities|Casting|CastToBP_Player OtherActor)
  (Audio|PlaySoundatLocation "/Game/SFX/Door.Door" "0, 0, 0" "0, 0, 0" 1.0 1.0 0.0 0 0 0 0)
  (Components|MoveComponentTo _cube (+ (Variables|/Script/Engine.SceneComponent|GetRelativeLocation _cube) "0.000000,0.000000,300.000000") (Variables|/Script/Engine.SceneComponent|GetRelativeRotation _cube) false false 1.0 false)
  (Components|DestroyComponent (Variables|Default|GetBox)))

(fn ConstructionScript)