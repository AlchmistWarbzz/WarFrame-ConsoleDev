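; BP_Weapon is the player's melee sword, handling its trail effect and hit damage against Moa body enemies and the Moa boss.
; Swordattack centers the FXSword trail between the mesh's top and bottom sockets, sets its width from their distance and activates it; Deactivate stops it.
; Box overlaps apply fixed damage while the player is attacking, with a separate DoOnce and short delay per enemy type limiting repeat hits.
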(event OnComponentEndOverlap(Box)
  (params (OverlappedComponent :type Primitive%20Component%20Object%20Reference) (OtherActor :type Actor%20Object%20Reference) (OtherComp :type Primitive%20Component%20Object%20Reference) (OtherBodyIndex :type Integer))
  ;[1 0 0] Cause Damage
)

(event OnComponentBeginOverlap(Box)
  (params (OverlappedComponent :type Primitive%20Component%20Object%20Reference) (OtherActor :type Actor%20Object%20Reference) (OtherComp :type Primitive%20Component%20Object%20Reference) (OtherBodyIndex :type Integer) (bFromSweep :type Boolean) (SweepResult :type Hit%20Result%20Structure%20%28by%20ref%29))
  ;[1 0 0] Cause Damage
  (if (Variables|/Game/Characters/Player/BP_Player.BP_Player_C|GetIsAttacking (Variables|Default|GetPlayerRef))
    (Utilities|FlowControl|Sequence
      (:then_0
        (bind _asbp_enemy_moa_body (Utilities|Casting|CastToBP_EnemyMoaBody OtherActor))
        (Utilities|FlowControl|DoOnce false :!label _label
          (:Completed
            (Game|Damage|ApplyDamage _asbp_enemy_moa_body 15.0 0 0)
            (Utilities|FlowControl|Delay 0.2)
            (goto _label Reset))))
      (:then_1
        (bind _asbp_moa_boss (Utilities|Casting|CastToBP_MoaBoss OtherActor))
        (Utilities|FlowControl|DoOnce false :!label _label_2
          (:Completed
            (Game|Damage|ApplyDamage _asbp_moa_boss 15.0 0 0)
            (Utilities|FlowControl|Delay 0.2)
            (goto _label_2 Reset)))))))

(event Custom|Sword%20attack
  (bind _staticmesh (Variables|Default|GetStaticMesh))
  (bind _fxsword (Variables|Default|GetFXSword))
  (bind _returnvalue (Transformation|GetSocketLocation _staticmesh "BottomSocket"))
  (bind _returnvalue_2 (Transformation|GetSocketLocation _staticmesh "TopSocket"))
  (bind _returnvalue_3 (- _returnvalue_2 _returnvalue))
  ;[0 1 0.1001] Spawn VFX
  (Transformation|SetWorldTransform _fxsword (Math|Transform|MakeTransform (/ (+ _returnvalue_2 _returnvalue) 2.0) (Math|Rotator|MakeRotfromZ _returnvalue_3) "1.000000,1.000000,1.000000") false false)
  (Effects|Components|ParticleSystem|SetFloatParameter _fxsword "TrailWidth" (Math|Vector|VectorLength _returnvalue_3))
  (Components|Activation|Activate (Variables|Default|GetFXSword) true))

(event Custom|Deactivate
  ;[1 0.4687 0] Deactivate
  (Components|Activation|Deactivate (Variables|Default|GetFXSword)))

(event EventBeginPlay
  ;[0.1121 0.5401 1] Reference BP
  (Utilities|FlowControl|Sequence
    (:then_0
      (Actor|GetActorOfClass "/Game/Characters/Moa/BP_EnemyMoaHead.BP_EnemyMoaHead_C")
      (Actor|GetActorOfClass "/Game/Characters/Moa/BP_EnemyMoaBody.BP_EnemyMoaBody_C")
      (Actor|GetActorOfClass "/Game/Characters/Moa/BP_MoaBoss.BP_MoaBoss_C")
      (bind _returnvalue (Actor|GetActorOfClass "/Game/Characters/Player/BP_Player.BP_Player_C"))
      (Variables|Default|SetPlayerRef _returnvalue))
    (:then_1
      (CallFunction|Deactivate))))

(event EventTick
  (params (DeltaSeconds :type Float%20%28single-precision%29)))

(fn ConstructionScript)