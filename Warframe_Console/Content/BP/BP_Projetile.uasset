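; BP_Projetile is a projectile that damages and slows the player on hit, and self-destructs five seconds after spawning.
; BeginPlay caches player and BP_EnemyMoa references, though only the player's is used.
; Overlap pauses into BP_PauseMenu if health is near zero; otherwise, touching the player's Box destroys the projectile and applies damage and slow.
; The projectile's own Tick restores player speed after a Delay, despite that destruction on hit.
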(event EventBeginPlay
  (bind _returnvalue (Actor|GetActorOfClass "/Game/Characters/Moa/BP_EnemyMoa.BP_EnemyMoa_C"))
  (Variables|Default|SetMoa%20Ref _returnvalue)
  ;[1 1 1] Ref for Blueprints
  (bind _returnvalue_2 (Actor|GetActorOfClass "/Game/Characters/Player/BP_Player.BP_Player_C"))
  (Variables|Default|SetPlayer%20Ref _returnvalue_2)
  (Utilities|FlowControl|Delay 5.0)
  (Actor|DestroyActor))

(event Collision|EventActorBeginOverlap
  (params (OtherActor :type Actor%20Object%20Reference))
  (bind _player_ref (Variables|Default|GetPlayer%20Ref))
  ;[1 1 1] Damage Player's Health
  (if (< (Variables|/Game/Characters/Player/BP_Player.BP_Player_C|GetPlayerHealth _player_ref) 0.01)
    (Game|SetGamePaused true)
    (bind _returnvalue (UserInterface|CreateWidget "/Game/BP/MainMenu/BP_PauseMenu.BP_PauseMenu_C"))
    (UserInterface|Viewport|AddtoViewport _returnvalue 0)
    (Variables|/Script/Engine.PlayerController|SetbShowMouseCursor (Game|GetPlayerController 0) true)
    (elif (Class|PrimitiveComponent|IsOverlappingComponent (Variables|/Game/Characters/Player/BP_Player.BP_Player_C|GetBox _player_ref) (Variables|Default|GetSphere))
      (Utilities|FlowControl|Sequence
        (:then_0
          (Actor|DestroyActor))
        (:then_1
          (Variables|/Game/Characters/Player/BP_Player.BP_Player_C|SetPlayerHealth _player_ref (- (Variables|/Game/Characters/Player/BP_Player.BP_Player_C|GetPlayerHealth _player_ref) 0.05))
          (bind _output_get (Variables|/Script/Engine.CharacterMovementComponent|SetMaxWalkSpeed (Variables|/Script/Engine.Character|GetCharacterMovement _player_ref) 2e+02))
          (Development|PrintString "Hit Player")
          (Development|PrintString (Utilities|String|ToString(Float) _output_get)))))))

(event EventTick
  (params (DeltaSeconds :type Float%20%28single-precision%29))
  (bind _player_ref (Variables|Default|GetPlayer%20Ref))
  (bind _charactermovement (Variables|/Script/Engine.Character|GetCharacterMovement _player_ref))
  (if (< (Variables|/Script/Engine.CharacterMovementComponent|GetMaxWalkSpeed _charactermovement) 5e+02)
    (Utilities|FlowControl|Delay 1.0)
    (Variables|/Script/Engine.CharacterMovementComponent|SetMaxWalkSpeed _charactermovement 8.5e+02)
    (else
      (Development|PrintString (Utilities|String|ToString(Float) (stale Collision|EventActorBeginOverlap _output_get))))))

(fn ConstructionScript)