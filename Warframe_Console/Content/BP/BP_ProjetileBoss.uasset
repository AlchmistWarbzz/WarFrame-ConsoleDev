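; BP_ProjetileBoss is a boss projectile that damages and slows the player on impact.
; On hit, it applies fixed damage to a BP_Player and lowers its max walk speed without restoring it here, then destroys itself whatever it struck.
; On BeginPlay, it attaches an FX_BeamTrail effect at the mesh's TrailSocket, feeding the socket's Z into BeamAlignment before activation.
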(event EventBeginPlay
  (bind _staticmesh (Variables|Default|GetstaticMesh))
  (bind _returnvalue (Transformation|GetSocketLocation _staticmesh "TrailSocket"))
  ;[1 1 1] VFX
  (bind _returnvalue_2 (Niagara|SpawnSystemAttached "/Game/VFX/FX_BeamTrail.FX_BeamTrail" _staticmesh "None" _returnvalue (Math|Rotator|MakeRotfromZ _returnvalue) "KeepWorldPosition" false false))
  (Effects|Components|ParticleSystem|SetFloatParameter _returnvalue_2 "BeamAlignment" (.Z (Class|KismetMathLibrary|BreakVector3f _returnvalue)))
  (Components|Activation|Activate _returnvalue_2 true))

(event EventTick
  (params (DeltaSeconds :type Float%20%28single-precision%29)))

(event Collision|EventHit
  (params (MyComp :type Primitive%20Component%20Object%20Reference) (Other :type Actor%20Object%20Reference) (OtherComp :type Primitive%20Component%20Object%20Reference) (bSelfMoved :type Boolean) (HitLocation :type Vector :default "0, 0, 0") (HitNormal :type Vector :default "0, 0, 0") (NormalImpulse :type Vector :default "0, 0, 0") (Hit :type Hit%20Result%20Structure%20%28by%20ref%29))
  ;[1 0 0] Damage Player
  (Utilities|FlowControl|Sequence
    (:then_0
      (bind _asbp_player (Utilities|Casting|CastToBP_Player Other))
      (Game|Damage|ApplyDamage _asbp_player 2e+01 0 0)
      ;;[1 0.4458 0] Slow Player down
      (Variables|/Script/Engine.CharacterMovementComponent|SetMaxWalkSpeed (Variables|/Script/Engine.Character|GetCharacterMovement _asbp_player) 2e+02))
    (:then_1
      (Actor|DestroyActor))))

(fn ConstructionScript)