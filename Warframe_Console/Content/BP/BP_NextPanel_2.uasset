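; Door actor that handles the player's exit from puzzle panel two to the next area.
; PanelTwoComplete blends the view to the player's CameraP4, raises the Cube door with a sound and disables collision on BP_CameraChange's Sphere3 and Box.
; When the player overlaps the Box, input is disabled while the door lowers, then the view blends to CameraP1 and the player teleports to the Teleport transform before regaining input.
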(event OnComponentBeginOverlap(Box)
  (params (OverlappedComponent :type Primitive%20Component%20Object%20Reference) (OtherActor :type Actor%20Object%20Reference) (OtherComp :type Primitive%20Component%20Object%20Reference) (OtherBodyIndex :type Integer) (bFromSweep :type Boolean) (SweepResult :type Hit%20Result%20Structure%20%28by%20ref%29))
  (bind _teleport (Variables|Default|GetTeleport))
  (bind _cube (Variables|Default|GetCube))
  (bind _asbp_player (Utilities|Casting|CastToBP_Player OtherActor))
  (bind _output_get (Variables|Default|SetAs%20BP%20Player _asbp_player))
  (Input|DisableInput _output_get 0)
  (Audio|PlaySoundatLocation "/Game/SFX/Door.Door" "0, 0, 0" "0, 0, 0" 1.0 1.0 0.0 0 0 0 0)
  (Components|MoveComponentTo _cube (- (Variables|/Script/Engine.SceneComponent|GetRelativeLocation _cube) "0.000000,0.000000,300.000000") (Variables|/Script/Engine.SceneComponent|GetRelativeRotation _cube) false false 1.0 false)
  (Utilities|FlowControl|Delay 1.0)
  (Game|Player|SetViewTargetwithBlend (Game|GetPlayerController 0) (Variables|/Game/Characters/Player/BP_Player.BP_Player_C|GetCameraP1 (Variables|Default|GetAs%20BP%20Player)) 0.5 "VTBlend_Linear" 0.0 false)
  (Transformation|SetActorLocationAndRotation (Variables|Default|GetAs%20BP%20Player) (Math|Transform|TransformLocation (Transformation|GetActorTransform) (.location _teleport)) (.rotation _teleport))
  (Input|EnableInput (Variables|Default|GetAs%20BP%20Player) 0))

(event Custom|PanelTwoComplete
  (bind _cube (Variables|Default|GetCube))
  (bind _returnvalue (Actor|GetActorOfClass "/Game/Characters/Player/BP_Player.BP_Player_C"))
  (Game|Player|SetViewTargetwithBlend (Game|GetPlayerController 0) (Variables|/Game/Characters/Player/BP_Player.BP_Player_C|GetCameraP4 _returnvalue) 0.5 "VTBlend_Linear" 0.0 false)
  (Audio|PlaySoundatLocation "/Game/SFX/Door.Door" "0, 0, 0" "0, 0, 0" 1.0 1.0 0.0 0 0 0 0)
  (Components|MoveComponentTo _cube (+ (Variables|/Script/Engine.SceneComponent|GetRelativeLocation _cube) "0.000000,0.000000,300.000000") (Variables|/Script/Engine.SceneComponent|GetRelativeRotation _cube) false false 1.0 false)
  (bind _returnvalue_2 (Actor|GetActorOfClass "/Game/BP/Cameras/BP_CameraChange.BP_CameraChange_C"))
  (Collision|SetCollisionEnabled (Variables|/Game/BP/Cameras/BP_CameraChange.BP_CameraChange_C|GetSphere3 _returnvalue_2) "NoCollision"))

(fn ConstructionScript)